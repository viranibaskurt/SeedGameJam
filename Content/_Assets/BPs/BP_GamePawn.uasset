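; BP_GamePawn is a pawn Blueprint that handles physics responses on its capsule for explode and reset events.
; ExplodeBP turns on capsule gravity, while ResetForces turns it off and toggles physics simulation off and on to clear motion.
; SetRagdollStateBP is empty; its skeletal mesh ragdoll and reattach-to-capsule logic is left disconnected and never runs.
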(event EventBeginPlay)

(event Collision|EventActorBeginOverlap
  (params (OtherActor :type Actor%20Object%20Reference)))

(event EventTick
  (params (DeltaSeconds :type Float%20%28single-precision%29)))

(event EventSetRagdollStateBP
  (params (State :type Boolean)))

(event EventExplodeBP
  (Physics|SetEnableGravity (Variables|Default|GetCapsule) true))

(event EventResetForces
  (Physics|SetEnableGravity (Variables|Default|GetCapsule) false)
  (Physics|SetSimulatePhysics (Variables|Default|GetCapsule) false)
  (Physics|SetSimulatePhysics (Variables|Default|GetCapsule) true))

(fn ConstructionScript)