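; Game mode that sets up a level with a controlled pawn and a spawned pool of repeating pawns, and manages its UI.
; BeginPlay caches the first PlayerStart location, shows the cursor and creates in-game and screen-change widgets.
; Events feed timer and self count to the HUD, swap in win or fail screens, and drive a timeline blur effect.
; An unconnected prototype records player input for replay on a second pawn.
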(event Custom|ResetInGameUi
  (bind _returnvalue (UserInterface|CreateWidget "/Game/_Assets/BPs/UI/WBP_InGame.WBP_InGame_C"))
  (bind _output_get (Variables|Default|SetInGameUI _returnvalue))
  (UserInterface|Viewport|AddtoViewport _output_get 0))

(event EventBeginPlay
  (Utilities|FlowControl|Sequence
    (:then_0
      (bind _asgame_pawn (Utilities|Casting|CastToGamePawn (Game|Player|GetPlayerPawn 0)))
      (Variables|Default|SetControlledPawn _asgame_pawn))
    (:then_1
      (for _index (range 0 4)
        (bind _returnvalue (Game|SpawnActorfromClass "/Game/_Assets/BPs/BP_GamePawn.BP_GamePawn_C" (Math|Transform|MakeTransform "0, 0, 0" "0, 0, 0" "1,1,1") "Undefined" 0 0))
        (Utilities|Array|Add (Variables|Default|GetRepeatingPawns) _returnvalue)))
    (:then_2
      (bind _outactors (Actor|GetAllActorsOfClass "/Script/Engine.PlayerStart"))
      (Variables|Default|SetStartLocation (Transformation|GetActorLocation (Utilities|Array|Get(acopy) _outactors))))
    (:then_3
      (CallFunction|ResetinGameUi))
    (:then_4
      (Variables|/Script/Engine.PlayerController|SetbShowMouseCursor (Game|GetPlayerController 0) true))
    (:then_5
      (bind _returnvalue_2 (UserInterface|CreateWidget "/Game/_Assets/BPs/UI/WBP_ScreenChange.WBP_ScreenChange_C"))
      (bind _output_get (Variables|Default|SetScreenChangeUI _returnvalue_2))
      (UserInterface|Viewport|AddtoViewport _output_get 0))))

(event EventTick
  (params (DeltaSeconds :type Float%20%28single-precision%29)))

(event EventInitNumSelfUI
  (params (Num :type Integer))
  (bind _ingameui (Variables|Default|GetInGameUI)
    (:then
      (Default|SetNumSelf _ingameui Num))
    (:else)))

(event EventShowFailUI
  (Viewport|RemoveAllWidgets)
  (bind _returnvalue (UserInterface|CreateWidget "/Game/_Assets/BPs/UI/WBP_EndGameFail.WBP_EndGameFail_C"))
  (UserInterface|Viewport|AddtoViewport _returnvalue 0))

(event EventInitTimerUI
  (params (Time :type Float%20%28single-precision%29))
  (bind _ingameui (Variables|Default|GetInGameUI)
    (:then
      (Default|SetTime _ingameui Time))
    (:else)))

(event EventShowHandEndScreenEffect
  (bind _newtrack_0 (Timeline|ScreenEffectTimeline PlayFromStart)
    (:Update
      (bind _screenchangeui (Variables|Default|GetScreenChangeUI)
        (:then
          (Default|SetBlurVal _screenchangeui _newtrack_0))
        (:else)))))

(event EventShowWinUI
  (Viewport|RemoveAllWidgets)
  (bind _returnvalue (UserInterface|CreateWidget "/Game/_Assets/BPs/UI/WBP_EndGameSuccess.WBP_EndGameSuccess_C"))
  (UserInterface|Viewport|AddtoViewport _returnvalue 0))

(fn ConstructionScript)